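; BP_Pawn is a pawn that reports which actor lies under the mouse cursor when clicked.
; BeginPlay shows the cursor on player controller 0.
; A left click runs a complex Visibility trace under the cursor and prints the hit actor's display name.
; Unconnected nodes for object-type hits, mouse position and screen-to-world deprojection remain in the event graph.
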(event `self.ReceiveBeginPlay`
  (set `PlayerController.bShowMouseCursor` true (`GameplayStatics.GetPlayerController` 0)))

(event `Key|LeftMouseButton`
  (params (Key :type "Key Structure"))
  (:`Pressed`
    (`KismetSystemLibrary.PrintString` (`KismetSystemLibrary.GetDisplayName` (`.HitActor` (`GameplayStatics.BreakHitResult` (`PlayerController.GetHitResultUnderCursorByChannel` (`GameplayStatics.GetPlayerController` 0) "TraceTypeQuery1" true)))))))

(fn `UserConstructionScript`)